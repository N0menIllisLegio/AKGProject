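; BP_PlayerController possesses the player pawn at startup and turns input into movement, camera look, jumping, interaction and attacks.
; Movement follows camera yaw, while jump applies a mass-independent impulse to the physics mesh after a vertical velocity check.
; E, F and Attack use BP_Player's trace to send an interact message, send a thrust message along camera forward, or damage a hit BP_NPC.
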(event EventBeginPlay
  (bind _self self)
  ;[1 1 1] Set pawn to variable and possess it
  (Variables|/Script/Engine.PlayerController|SetbShowMouseCursor _self false)
  (Input|SetInputModeGameOnly _self)
  (bind _output_get (Variables|Default|SetPlayerCharacter (Game|Player|GetPlayerPawn 0)))
  (Pawn|Possess _output_get)
  (Variables|Default|SetThurstPower 4e+02))

(event Input|ActionEvents|InputActionAttack
  (params (Key :type Key%20Structure :default "None"))
  ;[1 1 1] Attack
  (:Pressed
    (bind _asbp_player (Utilities|Casting|CastToBP_Player (Variables|Default|GetPlayerCharacter)))
    (bind (_ishitted _hitresult) (Default|Trace _asbp_player (Variables|/Game/Pawns/BP_Player.BP_Player_C|GetLaserDistance _asbp_player)))
    (if _ishitted
      (bind _asbp_npc (Utilities|Casting|CastToBP_NPC (.HitActor (Collision|BreakHitResult _hitresult))))
      (Default|TakeDamage _asbp_npc (Variables|/Game/Pawns/BP_Player.BP_Player_C|GetDamage _asbp_player)))))

(event Input|ActionEvents|InputActionJump
  (params (Key :type Key%20Structure :default "None"))
  (bind _playercharacter (Variables|Default|GetPlayerCharacter))
  ;[1 1 1] Jump
  ; (Only with physics ON)
  (:Pressed
    (if (Math|Float|InRange(Float) (.Z (Math|Vector|BreakVector (Transformation|GetVelocity _playercharacter))) -1.0 1.0)
      (bind _asbp_player (Utilities|Casting|CastToBP_Player _playercharacter))
      (Physics|AddImpulse (Variables|/Game/Pawns/BP_ParentPawn.BP_ParentPawn_C|GetSM_Pawn _asbp_player) "0.000000, 0,500.000000" "None" true) ; Ignoring wheight
    )))

(event Input|AxisEvents|InputAxisTurn
  (params (AxisValue :type Float%20%28single-precision%29))
  ;[1 1 1] Camera Movement
  (Pawn|Input|AddControllerYawInput (Variables|Default|GetPlayerCharacter) (/ AxisValue 2.0)))

(event Input|AxisEvents|InputAxisLookUp
  (params (AxisValue :type Float%20%28single-precision%29))
  ;[1 1 1] Camera Movement
  (Pawn|Input|AddControllerPitchInput (Variables|Default|GetPlayerCharacter) (/ AxisValue 2.0)))

(event Input|AxisEvents|InputAxisMoveX
  (params (AxisValue :type Float%20%28single-precision%29))
  ;[1 1 1] Character Movement
  (Pawn|Input|AddMovementInput (Variables|Default|GetPlayerCharacter) (Math|Vector|GetRightVector (Math|Rotator|MakeRotator 0.0 0.0 (.Yaw (Math|Rotator|BreakRotator (Pawn|GetControlRotation (Variables|Default|GetPlayerCharacter) :!class /Script/Engine.Pawn))))) (* AxisValue (Variables|Default|GetCurrentSpeed)) false))

(event Input|AxisEvents|InputAxisMoveY
  (params (AxisValue :type Float%20%28single-precision%29))
  ;[1 1 1] Character Movement
  (Pawn|Input|AddMovementInput (Variables|Default|GetPlayerCharacter) (Math|Vector|GetForwardVector (Math|Rotator|MakeRotator 0.0 0.0 (.Yaw (Math|Rotator|BreakRotator (Pawn|GetControlRotation (Variables|Default|GetPlayerCharacter) :!class /Script/Engine.Pawn))))) (* AxisValue (Variables|Default|GetCurrentSpeed)) false))

(event Input|KeyboardEvents|E
  (params (Key :type Key%20Structure :default "None"))
  ;[1 1 1] Interact E
  (:Pressed
    (bind _asbp_player (Utilities|Casting|CastToBP_Player (Variables|Default|GetPlayerCharacter)))
    (bind (_ishitted _hitresult) (Default|Trace _asbp_player 2e+02))
    (if _ishitted
      (bind _asbp_player_2 (Utilities|Casting|CastToBP_Player (Variables|Default|GetPlayerCharacter)))
      (Class|BPIInteraction|Interact(Message) (.HitActor (Collision|BreakHitResult _hitresult)) _asbp_player_2))))

(event Input|KeyboardEvents|F
  (params (Key :type Key%20Structure :default "None"))
  ;[1 1 1] Interact F
  (:Pressed
    (bind _asbp_player (Utilities|Casting|CastToBP_Player (Variables|Default|GetPlayerCharacter)))
    (bind (_ishitted _hitresult) (Default|Trace _asbp_player 2e+02))
    (if _ishitted
      (Class|BPIInteraction|Thrust(Message) (.HitActor (Collision|BreakHitResult _hitresult)) (Math|Vector|GetForwardVector (Variables|/Game/Pawns/BP_Player.BP_Player_C|GetCamera _asbp_player)) (Variables|Default|GetThurstPower) (Variables|/Game/Pawns/BP_Player.BP_Player_C|GetThrustDamage _asbp_player)))))

(fn ConstructionScript)