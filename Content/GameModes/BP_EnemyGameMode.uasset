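; Game mode for the enemy-elimination scenario: the player wins once no enemies remain and loses on death.
; BeginPlay extends the parent mode, sets a time limit and strips the hostage, bomb and timer widgets from the HUD.
; CheckConditions derives the game state from player survival and enemy count, with a Russian death message as defeat cause.
; Victory and Defeat show their own end-screen widgets.
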(event EventBeginPlay
  (bind _gamehudreference (Variables|Default|GetGameHUDReference))
  (|CallParentFunction)
  (Variables|Default|SetTimeLimit 1.8e+02)
  (Widget|RemovefromParent (Variables|/Game/HUDs/PlayerHUD.PlayerHUD_C|GetHostagesObjective _gamehudreference))
  (Widget|RemovefromParent (Variables|/Game/HUDs/PlayerHUD.PlayerHUD_C|GetBombObjective _gamehudreference))
  (Widget|RemovefromParent (Variables|/Game/HUDs/PlayerHUD.PlayerHUD_C|GetTimer _gamehudreference)))

(fn ConstructionScript
  (|CallParentFunction))

(fn Victory
  (bind _returnvalue (UserInterface|CreateWidget "/Game/HUDs/Enemies/EnemyVictoryHUD.EnemyVictoryHUD_C"))
  (UserInterface|Viewport|AddtoViewport _returnvalue 0)
  (return true))

(fn Defeat
  (params (CauseOfDefeat :type String))
  (Variables|Default|SetCauseOfDefeat CauseOfDefeat)
  (bind _returnvalue (UserInterface|CreateWidget "/Game/HUDs/Enemies/EnemyDefeatHUD.EnemyDefeatHUD_C"))
  (UserInterface|Viewport|AddtoViewport _returnvalue 0)
  (return true))

(fn CheckConditions
  (if (Variables|Default|GetPlayerAlive)
    (if (> (Variables|Default|GetEnemiesAlive) 0)
      (return "NewEnumerator2" "")
      (else
        (return "NewEnumerator0" "")))
    (else
      (return "NewEnumerator1" "Вы погибли"))))