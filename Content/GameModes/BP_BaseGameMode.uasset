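; Base game mode that sets up the match HUD and tracks victory or defeat in a hostage-and-enemy game.
; BeginPlay counts BP_Enemy and BP_Hostage actors into total and alive variables, then creates and displays the PlayerHUD.
; Every Tick polls CheckConditions and calls Victory, or Defeat with its cause.
; These three functions are placeholders, with CheckConditions always returning ContinueGame, leaving the actual rules to child game modes.
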(event EventBeginPlay
  ;[1 1 1] Get Hostages/Enemies and Set HUD
  (Utilities|FlowControl|Sequence
    (:then_0
      (bind _outactors (Actor|GetAllActorsOfClass "/Game/Characters/BP_Enemy.BP_Enemy_C"))
      (bind _output_get (Variables|Default|SetEnemiesAlive (Utilities|Array|Length _outactors)))
      (Variables|Default|SetTotalEnemies _output_get))
    (:then_1
      (bind _outactors_2 (Actor|GetAllActorsOfClass "/Game/Characters/BP_Hostage.BP_Hostage_C"))
      (bind _output_get_2 (Variables|Default|SetTotalHostages (Utilities|Array|Length _outactors_2)))
      (Variables|Default|SetHostagesAlive _output_get_2))
    (:then_2
      (bind _returnvalue (UserInterface|CreateWidget "/Game/HUDs/PlayerHUD.PlayerHUD_C"))
      (bind _output_get_3 (Variables|Default|SetGameHUDReference _returnvalue))
      (UserInterface|Viewport|AddtoViewport _output_get_3 0))))

(event EventTick
  (params (DeltaSeconds :type Float%20%28single-precision%29))
  ;[1 1 1] CheckConditions
  (bind (_gamestate _causeofdefeat) (CallFunction|CheckConditions))
  (switch Utilities|FlowControl|Switch|SwitchonCheckConditionEnum _gamestate
    (:NewEnumerator0
      (CallFunction|Victory))
    (:NewEnumerator1
      (CallFunction|Defeat _causeofdefeat))))

(fn ConstructionScript)

(fn Victory
  (return true))

(fn Defeat
  (params (CauseOfDefeat :type String))
  (return true))

(fn CheckConditions
  (return "NewEnumerator2" ""))