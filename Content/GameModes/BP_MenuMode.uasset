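; BP_MenuMode is the menu game mode, which restores saved sound settings and shows the menu HUD on BeginPlay.
; A GameStarted flag on BP_GameInstance limits the load to once per game instance, copying Sounds from the BP_SaveSound in the "Sounds" slot.
; The menu widget is then created and added to the viewport on every BeginPlay where the BP_GameInstance cast succeeds.
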(event EventBeginPlay
  (bind _asbp_game_instance (Utilities|Casting|CastToBP_GameInstance (Game|GetGameInstance)))
  (if (Variables|/Game/BP_GameInstance.BP_GameInstance_C|GetGameStarted _asbp_game_instance)
    _
    (else
      (bind _returnvalue (SaveGame|LoadGamefromSlot "Sounds"))
      (bind _asbp_save_sound (Utilities|Casting|CastToBP_SaveSound _returnvalue)
        (:then
          (Variables|/Game/BP_GameInstance.BP_GameInstance_C|SetSounds _asbp_game_instance (Variables|/Game/BP_SaveSound.BP_SaveSound_C|GetSounds _asbp_save_sound)))
        (:CastFailed
          _))
      (Variables|/Game/BP_GameInstance.BP_GameInstance_C|SetGameStarted _asbp_game_instance true)))
  (bind _returnvalue_2 (UserInterface|CreateWidget "/Game/HUDs/MenuHUD.MenuHUD_C"))
  (UserInterface|Viewport|AddtoViewport _returnvalue_2 0))

(fn ConstructionScript)