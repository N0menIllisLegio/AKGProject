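; Tutorial game mode that keeps one enemy and one hostage present in the level for practice.
; BeginPlay caches spawn and patrol marker actors, spawns both AI with their behavior trees, removes the HUD objectives and timer, and hands the bomb to the HUD.
; Tick watches both references and, when one is invalid, starts a single delayed respawn timer guarded by a flag.
; Spawn functions only spawn if none of that class exists.
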(event EventBeginPlay
  (bind _gamehudreference (Variables|Default|GetGameHUDReference))
  (|CallParentFunction)
  (Utilities|FlowControl|Sequence
    (:then_0
      (bind _returnvalue (Actor|GetActorOfClass "/Game/Maps/TutorialLevel/EnemySpawnTP.EnemySpawnTP_C"))
      (Variables|Default|SetEnemySpawnPoint _returnvalue))
    (:then_1
      (bind _returnvalue_2 (Actor|GetActorOfClass "/Game/Maps/TutorialLevel/HostageSpawnTP.HostageSpawnTP_C"))
      (Variables|Default|SetHostageSpawnPoint _returnvalue_2))
    (:then_2
      (bind _outactors (Actor|GetAllActorsOfClass "/Game/Maps/TutorialLevel/PatrolTP.PatrolTP_C"))
      (Variables|Default|SetPatrolStart (Utilities|Array|Get(acopy) _outactors))
      (Variables|Default|SetPatrolEnd (Utilities|Array|Get(acopy) _outactors 1)))
    (:then_3
      (CallFunction|SpawnEnemy)
      (CallFunction|SpawnHostage))
    (:then_4
      (Widget|RemovefromParent (Variables|/Game/HUDs/PlayerHUD.PlayerHUD_C|GetObjectives _gamehudreference))
      (Widget|RemovefromParent (Variables|/Game/HUDs/PlayerHUD.PlayerHUD_C|GetTimer _gamehudreference)))
    (:then_5
      (bind _returnvalue_3 (Actor|GetActorOfClass "/Game/Actors/BP_Bomb.BP_Bomb_C"))
      (Variables|/Game/HUDs/PlayerHUD.PlayerHUD_C|SetBomb (Variables|Default|GetGameHUDReference) _returnvalue_3))))

(event EventTick
  (params (DeltaSeconds :type Float%20%28single-precision%29))
  (|CallParentFunction DeltaSeconds)
  (Utilities|FlowControl|Sequence
    (:then_0
      (Utilities|IsValid (Variables|Default|GetHostage)
        (:Is%20Valid
          (Variables|Default|SetSpawningHostage false))
        (:Is%20Not%20Valid
          (if (not (Variables|Default|GetSpawningHostage))
            (Utilities|Time|SetTimerbyFunctionName 0 "SpawnHostage" 1e+01)
            (Variables|Default|SetSpawningHostage true)))))
    (:then_1
      (Utilities|IsValid (Variables|Default|GetEnemy)
        (:Is%20Valid
          (Variables|Default|SetSpawningEnemy false))
        (:Is%20Not%20Valid
          (if (not (Variables|Default|GetSpawningEnemy))
            (Utilities|Time|SetTimerbyFunctionName 0 "SpawnEnemy" 1e+01)
            (Variables|Default|SetSpawningEnemy true)))))))

(fn ConstructionScript
  (|CallParentFunction))

(fn SpawnEnemy
  (bind _outactors (Actor|GetAllActorsOfClass "/Game/Characters/BP_Enemy.BP_Enemy_C"))
  (if (== (Utilities|Array|Length _outactors) 0)
    (bind _returnvalue (AI|SpawnAIFromClass "/Game/Characters/BP_Enemy.BP_Enemy_C" "/Game/Characters/AI/Enemy/BT_Enemy.BT_Enemy" (Transformation|GetActorLocation (Variables|Default|GetEnemySpawnPoint)) (Transformation|GetActorRotation (Variables|Default|GetEnemySpawnPoint)) false))
    (bind _asbp_enemy (Utilities|Casting|CastToBP_Enemy _returnvalue))
    (bind _output_get (Variables|Default|SetEnemy _asbp_enemy))
    (Variables|/Game/Characters/BP_Enemy.BP_Enemy_C|SetAFK _output_get (Variables|Default|GetEnemyStatus))
    (Variables|/Game/Characters/BP_Enemy.BP_Enemy_C|SetStartOfPatrolRoute _output_get (Variables|Default|GetPatrolStart))
    (Variables|/Game/Characters/BP_Enemy.BP_Enemy_C|SetEndOfPatrolRoute _output_get (Variables|Default|GetPatrolEnd))))

(fn SpawnHostage
  (bind _hostagespawnpoint (Variables|Default|GetHostageSpawnPoint))
  (bind _outactors (Actor|GetAllActorsOfClass "/Game/Characters/BP_Hostage.BP_Hostage_C"))
  (if (== (Utilities|Array|Length _outactors) 0)
    (bind _returnvalue (AI|SpawnAIFromClass "/Game/Characters/BP_Hostage.BP_Hostage_C" "/Game/Characters/AI/Hostage/BT_Hostage.BT_Hostage" (Transformation|GetActorLocation _hostagespawnpoint) (Transformation|GetActorRotation _hostagespawnpoint) false))
    (bind _asbp_hostage (Utilities|Casting|CastToBP_Hostage _returnvalue))
    (bind _output_get (Variables|Default|SetHostage _asbp_hostage))
    (Variables|/Game/Characters/BP_Hostage.BP_Hostage_C|SetStartPosition _output_get _hostagespawnpoint)))