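; Game mode for the bomb-defusal scenario, overriding the win, loss and condition logic of a parent game mode.
; On BeginPlay it takes its time limit from the level's BP_Bomb, passes that bomb to the HUD and removes the enemy and hostage objectives.
; CheckConditions derives the game state from player death, defusal and explosion, with Russian defeat causes.
; Victory and Defeat each show their own bomb-specific end-screen widget.
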(event EventBeginPlay
  (bind _gamehudreference (Variables|Default|GetGameHUDReference))
  (|CallParentFunction)
  (Utilities|FlowControl|Sequence
    (:then_0
      ;[1 1 1] Get Bomb Timer
      (bind _returnvalue (Actor|GetActorOfClass "/Game/Actors/BP_Bomb.BP_Bomb_C"))
      (Variables|Default|SetTimeLimit (Variables|/Game/Actors/BP_Bomb.BP_Bomb_C|GetTimer _returnvalue))
      (Variables|/Game/HUDs/PlayerHUD.PlayerHUD_C|SetBomb _gamehudreference _returnvalue))
    (:then_1
      (Widget|RemovefromParent (Variables|/Game/HUDs/PlayerHUD.PlayerHUD_C|GetEnemiesObjective _gamehudreference))
      (Widget|RemovefromParent (Variables|/Game/HUDs/PlayerHUD.PlayerHUD_C|GetHostagesObjective _gamehudreference)))))

(fn ConstructionScript
  (|CallParentFunction))

(fn Defeat
  (params (CauseOfDefeat :type String))
  (Variables|Default|SetCauseOfDefeat CauseOfDefeat)
  (bind _returnvalue (UserInterface|CreateWidget "/Game/HUDs/Bomb/BombDefeatHUD.BombDefeatHUD_C"))
  (UserInterface|Viewport|AddtoViewport _returnvalue 0)
  (return true))

(fn Victory
  (bind _returnvalue (UserInterface|CreateWidget "/Game/HUDs/Bomb/BombVictoryHUD.BombVictoryHUD_C"))
  (UserInterface|Viewport|AddtoViewport _returnvalue 0)
  (return true))

(fn CheckConditions
  (if (Variables|Default|GetPlayerAlive)
    (if (not (Variables|Default|GetBombDiffused))
      (if (not (Variables|Default|GetBombExploded))
        (return "NewEnumerator2" "")
        (else
          (return "NewEnumerator1" "Бомба взорвалась")))
      (else
        (return "NewEnumerator0" "")))
    (else
      (return "NewEnumerator1" "Вы погибли"))))