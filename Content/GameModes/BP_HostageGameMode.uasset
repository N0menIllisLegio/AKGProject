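; BP_HostageGameMode is the game mode for hostage rescue missions, overriding setup, condition checks and end screens from a parent mode.
; BeginPlay sets a time limit, then strips the enemy, bomb and timer widgets from the HUD.
; CheckConditions returns a game state with a Russian defeat reason: player death or no living hostages loses, all hostages rescued wins.
; Victory and Defeat each display their hostage-specific end screen.
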(event EventBeginPlay
  (bind _gamehudreference (Variables|Default|GetGameHUDReference))
  (|CallParentFunction)
  (Variables|Default|SetTimeLimit 1.8e+02)
  (Widget|RemovefromParent (Variables|/Game/HUDs/PlayerHUD.PlayerHUD_C|GetEnemiesObjective _gamehudreference))
  (Widget|RemovefromParent (Variables|/Game/HUDs/PlayerHUD.PlayerHUD_C|GetBombObjective _gamehudreference))
  (Widget|RemovefromParent (Variables|/Game/HUDs/PlayerHUD.PlayerHUD_C|GetTimer _gamehudreference)))

(fn ConstructionScript
  (|CallParentFunction))

(fn Victory
  (bind _returnvalue (UserInterface|CreateWidget "/Game/HUDs/Hostages/HostageVictoryHUD.HostageVictoryHUD_C"))
  (UserInterface|Viewport|AddtoViewport _returnvalue 0)
  (return true))

(fn Defeat
  (params (CauseOfDefeat :type String))
  (Variables|Default|SetCauseOfDefeat CauseOfDefeat)
  (bind _returnvalue (UserInterface|CreateWidget "/Game/HUDs/Hostages/HostageDefeatHUD.HostageDefeatHUD_C"))
  (UserInterface|Viewport|AddtoViewport _returnvalue 0)
  (return true))

(fn CheckConditions
  (if (Variables|Default|GetPlayerAlive)
    (if (== (Variables|Default|GetResquedHostages) (Variables|Default|GetTotalHostages))
      (return "NewEnumerator0" "")
      (elif (<= (Variables|Default|GetHostagesAlive) 0)
        (return "NewEnumerator1" "Все заложники мертвы")
        (else
          (return "NewEnumerator2" ""))))
    (else
      (return "NewEnumerator1" "Вы погибли"))))