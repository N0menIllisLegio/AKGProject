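; Player pawn with health and damage stats that shows a laser beam along the control rotation.
; Each tick it applies movement input scaled by delta time without sweep, and drives a dynamic material's Alpha from lost health.
; A line trace macro, duplicated by an unused Trace function, sets the beam's end at the hit point or maximum range.
; On Die it clears the game mode's PlayerAlive flag.
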(event EventBeginPlay
  ;[1 1 1] Event begin play
  (|CallParentFunction)
  (Variables|Default|SetLaserDistance 1e+03)
  (bind _output_get (Variables|Default|SetFullHealth 2e+02))
  (Variables|Default|SetCurrentHealth _output_get)
  (Variables|Default|SetName "Player")
  (Variables|Default|SetDamage 5e+01)
  (Variables|Default|SetThrustDamage 1e+01))

(event Collision|EventActorBeginOverlap
  (params (OtherActor :type Actor%20Object%20Reference))
  (|CallParentFunction OtherActor))

(event EventDie
  (bind _asbp_game_mode (Utilities|Casting|CastToBP_GameMode (Game|GetGameMode)))
  (Variables|/Game/BP_GameMode.BP_GameMode_C|SetPlayerAlive _asbp_game_mode false))

(event EventTick
  (params (DeltaSeconds :type Float%20%28single-precision%29))
  (|CallParentFunction DeltaSeconds)
  (bind _returnvalue (Class|Pawn|ConsumeMovementInputVector))
  (Transformation|AddActorWorldOffset (* _returnvalue DeltaSeconds))
  (CallFunction|ChangeColor)
  (bind (_ishitted _hitresult) (Utilities|TraceMacro (Variables|Default|GetLaserDistance))
    (:Out
      (CallFunction|DrawLaser _ishitted (.ImpactPoint (Collision|BreakHitResult _hitresult)) (Variables|Default|GetLaserDistance)))))

(fn ConstructionScript
  (|CallParentFunction))

(fn ChangeColor
  (Rendering|Material|SetScalarParameterValue (Variables|Default|GetDynamicMaterial) "Alpha" (- 1.0 (/ (Variables|Default|GetCurrentHealth) (Variables|Default|GetFullHealth))) :!class /Script/Engine.MaterialInstanceDynamic))

(fn Trace
  (params (TraceDistance :type Float%20%28single-precision%29))
  (bind _returnvalue (Transformation|GetActorLocation))
  (bind (_outhit _returnvalue_2) (Collision|LineTraceByChannel _returnvalue (+ _returnvalue (* (Math|Vector|GetForwardVector (Pawn|GetControlRotation :!class /Script/Engine.Pawn)) TraceDistance)) "TraceTypeQuery2" false 0 "None"))
  (return _returnvalue_2 _outhit))

(fn DrawLaser
  (params (IsHitted :type Boolean) (ImpactLocation :type Vector) (DefaultLaserDistance :type Float%20%28single-precision%29))
  (bind _sm_pawn (Variables|Default|GetSM_Pawn))
  (bind _laserbeam (Variables|Default|GetLaserBeam))
  (bind _returnvalue (Transformation|GetWorldLocation _sm_pawn))
  (if IsHitted
    (LocalVariables|SetTargetPoint ImpactLocation)
    (else
      (LocalVariables|SetTargetPoint (+ _returnvalue (* (Math|Vector|GetForwardVector (Pawn|GetControlRotation :!class /Script/Engine.Pawn)) DefaultLaserDistance)))))
  (Class|ParticleSystemComponent|SetBeamSourcePoint _laserbeam 0 _returnvalue)
  (Class|ParticleSystemComponent|SetBeamTargetPoint _laserbeam 0 (LocalVariables|GetTargetPoint)))