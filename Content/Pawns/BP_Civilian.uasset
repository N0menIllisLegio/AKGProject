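; BP_Civilian is a civilian NPC pawn built on a parent class that supplies its base begin-play and death behavior.
; On begin play it starts at full health, sets its name and assigns an NPC group on its HUD.
; When it dies, it clears the all-civilians-alive flag on BP_GameMode before running the parent death logic, which is skipped if the game mode cast fails.
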(event EventBeginPlay
  (|CallParentFunction)
  (bind _output_get (Variables|Default|SetFullHealth 1.0))
  (Variables|Default|SetCurrentHealth _output_get)
  (Variables|Default|SetName "Civilian")
  (Variables|/Game/HUDs/NpcHUD.NpcHUD_C|SetNpcGroup (Variables|Default|GetHUD) "NewEnumerator1"))

(event Collision|EventActorBeginOverlap
  (params (OtherActor :type Actor%20Object%20Reference))
  (|CallParentFunction OtherActor) ; This node is disabled and will not be called.\nDrag off pins to build functionality.
)

(event EventTick
  (params (DeltaSeconds :type Float%20%28single-precision%29))
  (|CallParentFunction DeltaSeconds) ; This node is disabled and will not be called.\nDrag off pins to build functionality.
)

(event EventDie
  (bind _asbp_game_mode (Utilities|Casting|CastToBP_GameMode (Game|GetGameMode)))
  (Variables|/Game/BP_GameMode.BP_GameMode_C|SetAllCiviliansAlive _asbp_game_mode false)
  (|CallParentFunction))

(fn ConstructionScript
  (|CallParentFunction))