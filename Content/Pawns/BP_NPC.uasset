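; NPC pawn with an on-screen widget and a physical reaction to being thrust.
; On BeginPlay it hands itself and a default group to its NpcHUD widget.
; Every tick it multi-line-traces on the Visibility channel toward the first player's pawn, showing the widget if a BP_Player is among the hits.
; Thrust applies a mass-independent impulse to the SMPawn mesh, then applies damage.
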(event EventBeginPlay
  ;[1 1 1] BeginPlay
  (|CallParentFunction)
  (bind _asnpc_hud (Utilities|Casting|CastToNpcHUD (UserInterface|GetUserWidgetObject (Variables|Default|GetNPCUI))))
  (bind _output_get (Variables|Default|SetHUD _asnpc_hud))
  (Variables|/Game/HUDs/NpcHUD.NpcHUD_C|SetNPC _output_get self)
  (Variables|/Game/HUDs/NpcHUD.NpcHUD_C|SetNpcGroup _output_get "NewEnumerator0"))

(event Collision|EventActorBeginOverlap
  (params (OtherActor :type Actor%20Object%20Reference))
  (|CallParentFunction OtherActor) ; This node is disabled and will not be called.\nDrag off pins to build functionality.
)

(event EventTick
  (params (DeltaSeconds :type Float%20%28single-precision%29))
  (|CallParentFunction DeltaSeconds)
  (CallFunction|WidgetVisibilitytoPlayer))

(event EventThrust
  (params (Direction :type Vector :default "0, 0, 0") (Power :type Float%20%28single-precision%29) (Damage :type Float%20%28single-precision%29))
  (Physics|AddImpulse (Variables|Default|GetSM_Pawn) (* Direction Power) "None" true) ; Ignoring wheight
  (CallFunction|TakeDamage Damage))

(fn ConstructionScript
  (|CallParentFunction))

(fn WidgetVisibilitytoPlayer
  (bind _npcui (Variables|Default|GetNPCUI))
  (bind _outhits (Collision|MultiLineTraceByChannel (Transformation|GetWorldLocation (Variables|Default|GetSM_Pawn)) (Transformation|GetActorLocation (Game|Player|GetPlayerPawn 0)) "TraceTypeQuery1" false 0 "None"))
  (bind _array_element (Utilities|Array|ForEachLoopwithBreak _outhits :!label _label)
    (:LoopBody
      (Utilities|Casting|CastToBP_Player (.HitActor (Collision|BreakHitResult _array_element))
        (:then
          (Rendering|SetVisibility _npcui true false)
          (goto _label Break))
        (:CastFailed
          (Rendering|SetVisibility _npcui false false))))))