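; Enemy pawn that damages the player when it detects them, extending a parent class that it configures with health, name, damage and HUD group.
; Each tick, TraceCone approximates a vision cone with scaled box traces stepped along the negative right vector.
; A detected player goes to CheckVision, which line-traces between meshes and applies damage on player hits.
; Death decrements the game mode's enemy count; the single-box Trace is unused.
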(event EventBeginPlay
  (|CallParentFunction)
  (bind _output_get (Variables|Default|SetFullHealth 1.5e+02))
  (Variables|Default|SetCurrentHealth _output_get)
  (Variables|Default|SetName "Enemy")
  (Variables|/Game/HUDs/NpcHUD.NpcHUD_C|SetNpcGroup (Variables|Default|GetHUD) "NewEnumerator2")
  (Variables|Default|SetDamage 1.0)
  (Variables|Default|SetTraceDistance -1e+03))

(event Collision|EventActorBeginOverlap
  (params (OtherActor :type Actor%20Object%20Reference))
  (|CallParentFunction OtherActor))

(event EventTick
  (params (DeltaSeconds :type Float%20%28single-precision%29))
  (|CallParentFunction DeltaSeconds)
  (CallFunction|TraceCone 0.0))

(event EventDie
  (bind _asbp_game_mode (Utilities|Casting|CastToBP_GameMode (Game|GetGameMode)))
  (Math|Integer|DecrementInt (Variables|/Game/BP_GameMode.BP_GameMode_C|GetEnemiesCount _asbp_game_mode)
    (:%20%20
      (|CallParentFunction))))

(fn ConstructionScript
  (|CallParentFunction))

(fn Trace
  (params (TraceDistance :type Float%20%28single-precision%29))
  (bind _returnvalue (Transformation|GetActorLocation))
  (bind _outhit (Class|KismetSystemLibrary|BoxTraceSingleforObjects _returnvalue (+ _returnvalue (* (Transformation|GetActorRightVector) TraceDistance)) "40.000000,40.000000,40.000000" "0, 0, 0" (Utilities|Array|MakeArray "ObjectTypeQuery4" "ObjectTypeQuery1") false 0 "None" true))
  (bind _asbp_player (Utilities|Casting|CastToBP_Player (.HitActor (Collision|BreakHitResult _outhit))))
  (Default|TakeDamage _asbp_player (Variables|Default|GetDamage)))

(fn TraceCone
  (params (TraceDistance :type Float%20%28single-precision%29))
  (bind _output_get (LocalVariables|SetBoxSide 5e+01))
  (bind _output_get_2 (LocalVariables|SetBoxLocation (Transformation|GetActorLocation)))
  (bind _outhits (Class|KismetSystemLibrary|BoxTraceMulti _output_get_2 (+ _output_get_2 "1.000000,1.000000,1.000000") (Math|Conversions|ToVector(Float) _output_get) "0, 0, 0" "TraceTypeQuery1" false 0 "None" true))
  (for _array_element _outhits
    (bind _asbp_player (Utilities|Casting|CastToBP_Player (.HitActor (Collision|BreakHitResult _array_element))))
    (CallFunction|CheckVision _asbp_player)
    (return))
  (for _index (range 0 2)
    (bind _output_get_3 (LocalVariables|SetBoxLocation (+ (LocalVariables|GetBoxLocation) (* (Transformation|GetActorRightVector) (* -1.0 (+ (LocalVariables|GetBoxSide) (* (LocalVariables|GetBoxSide) (LocalVariables|GetScaleValue))))))))
    (bind _output_get_4 (LocalVariables|SetBoxSide (* (LocalVariables|GetBoxSide) (LocalVariables|GetScaleValue))))
    (bind _outhits_2 (Class|KismetSystemLibrary|BoxTraceMulti _output_get_3 (+ _output_get_3 "1.000000,1.000000,1.000000") (Math|Conversions|ToVector(Float) _output_get_4) "0, 0, 0" "TraceTypeQuery1" false 0 "None" true))
    (for _array_element_2 _outhits_2
      (bind _asbp_player_2 (Utilities|Casting|CastToBP_Player (.HitActor (Collision|BreakHitResult _array_element_2))))
      (CallFunction|CheckVision _asbp_player_2)
      (return))))

(fn CheckVision
  (params (PlayerRef :type BP%20Player%20Object%20Reference))
  (bind _outhits (Collision|MultiLineTraceByChannel (Transformation|GetWorldLocation (Variables|Default|GetSM_Pawn)) (Transformation|GetWorldLocation (Variables|/Game/Pawns/BP_ParentPawn.BP_ParentPawn_C|GetSM_Pawn PlayerRef)) "TraceTypeQuery1" false 0 "None"))
  (bind _array_element (Utilities|Array|ForEachLoopwithBreak _outhits)
    (:LoopBody
      (bind _asbp_player (Utilities|Casting|CastToBP_Player (.HitActor (Collision|BreakHitResult _array_element))))
      (Default|TakeDamage _asbp_player (Variables|Default|GetDamage)))))