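; BP_ParentPawn is a base pawn that gives characters a simple health pool with damage, healing and death.
; BeginPlay fills health to its maximum, TakeDamage subtracts from it and calls Die at zero or below, which destroys the actor.
; Heal adds health, capped at the maximum.
; The construction script creates and stores a dynamic material instance from the SMPawn mesh, though nothing here modifies it.
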(event EventBeginPlay
  (bind _output_get (Variables|Default|SetFullHealth 1.5e+02))
  (Variables|Default|SetCurrentHealth _output_get))

(event Collision|EventActorBeginOverlap
  (params (OtherActor :type Actor%20Object%20Reference)))

(event EventTick
  (params (DeltaSeconds :type Float%20%28single-precision%29)))

(fn ConstructionScript
  (bind _returnvalue (Rendering|Material|CreateDynamicMaterialInstance (Variables|Default|GetSM_Pawn) 0 0 "None" :!class /Script/Engine.PrimitiveComponent))
  (Variables|Default|SetDynamicMaterial _returnvalue))

(fn TakeDamage
  (params (Damage :type Float%20%28single-precision%29))
  (bind _output_get (Variables|Default|SetCurrentHealth (- (Variables|Default|GetCurrentHealth) Damage)))
  (if (<= _output_get 0.0)
    (CallFunction|Die)))

(fn Die
  (Actor|DestroyActor))

(fn Heal
  (params (HP :type Float%20%28single-precision%29))
  (Variables|Default|SetCurrentHealth (Math|Float|Min(Float) (+ HP (Variables|Default|GetCurrentHealth)) (Variables|Default|GetFullHealth))))