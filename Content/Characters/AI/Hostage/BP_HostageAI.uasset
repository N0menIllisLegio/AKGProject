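; BP_HostageAI is the AI controller for hostage characters, running BT_Hostage on BeginPlay.
; Perception updates are routed by actor type to NoticedEnemy, which is an empty stub, or NoticedPlayer.
; NoticedPlayer writes the player's sighted state and location to the Blackboard and resets the CheckedLastPlayerPos flag on every update, including sight loss.
; A Focusing helper wraps SetFocus on a given actor.
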(event OnTargetPerceptionUpdated(AIPerception)
  (params (Actor :type Actor%20Object%20Reference) (Stimulus :type AI%20Stimulus%20Structure))
  (bind _asbp_enemy (Utilities|Casting|CastToBP_Enemy Actor)
    (:then
      (CallFunction|NoticedEnemy _asbp_enemy Stimulus))
    (:CastFailed
      (bind _asbp_player (Utilities|Casting|CastToBP_Player Actor))
      (CallFunction|NoticedPlayer _asbp_player Stimulus))))

(event EventBeginPlay
  (AI|RunBehaviorTree "/Game/Characters/AI/Hostage/BT_Hostage.BT_Hostage"))

(fn ConstructionScript)

(fn NoticedEnemy
  (params (Enemy :type BP%20Enemy%20Object%20Reference) (Stimulus :type AI%20Stimulus%20Structure)))

(fn NoticedPlayer
  (params (Player :type BP%20Player%20Object%20Reference) (Stimulus :type AI%20Stimulus%20Structure))
  (bind _returnvalue (AI|GetBlackboard 0))
  (AI|Components|Blackboard|SetValueasBool _returnvalue (Utilities|Name|MakeLiteralName "IsPlayerInSight") (.bSuccessfullySensed (Utilities|Struct|BreakAIStimulus Stimulus)))
  (AI|Components|Blackboard|SetValueasBool _returnvalue (Utilities|Name|MakeLiteralName "CheckedLastPlayerPos") false)
  (AI|Components|Blackboard|SetValueasVector _returnvalue (Utilities|Name|MakeLiteralName "PlayerLastLocation") (Transformation|GetActorLocation Player)))

(fn Focusing
  (params (Actor :type Actor%20Object%20Reference))
  (AI|SetFocus Actor))