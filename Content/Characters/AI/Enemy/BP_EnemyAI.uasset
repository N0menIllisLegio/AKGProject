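; AI controller for enemy characters that runs BT_Enemy and reacts to perceived players and hostages.
; Perception updates write sight, spotted and last-location blackboard keys, treating "Noise" stimuli separately, and Tick clears hostage sight when the stored hostage is invalid.
; Helpers turn the pawn, sphere-trace line of fire from the Glock to the player, and line-trace close-range hits, setting a timer-reset hitting flag.
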(event OnTargetPerceptionUpdated(AIPerception)
  (params (Actor :type Actor%20Object%20Reference) (Stimulus :type AI%20Stimulus%20Structure))
  (bind _asbp_player (Utilities|Casting|CastToBP_Player Actor)
    (:then
      (CallFunction|PlayerSpotted _asbp_player Stimulus))
    (:CastFailed
      (bind _asbp_hostage (Utilities|Casting|CastToBP_Hostage Actor))
      (CallFunction|HostageSpotted Stimulus _asbp_hostage))))

(event Custom|LookRight
  (Class|Actor|AddActorWorldRotation (Pawn|GetControlledPawn) "0,5.000000, 0")
  (Variables|Default|SetRotationYaw 5.0))

(event Custom|LookLeft
  (Class|Actor|AddActorWorldRotation (Pawn|GetControlledPawn) "0,-5.000000, 0")
  (Variables|Default|SetRotationYaw -5.0))

(event Custom|StopRotation
  (Variables|Default|SetRotationYaw 0.0))

(event EventBeginPlay
  (AI|RunBehaviorTree "/Game/Characters/AI/Enemy/BT_Enemy.BT_Enemy"))

(event EventTick
  (params (DeltaSeconds :type Float%20%28single-precision%29))
  (Utilities|IsValid (Variables|Default|GetHostage)
    (:Is%20Not%20Valid
      (AI|Components|Blackboard|SetValueasBool (AI|GetBlackboard 0) (Utilities|Name|MakeLiteralName "CanSeeHostage") false))))

(fn ConstructionScript)

(fn PlayerSpotted
  (params (Player :type BP%20Player%20Object%20Reference) (Stimulus :type AI%20Stimulus%20Structure))
  (bind (_age _expirationage _strength _stimuluslocation _receiverlocation _tag _bsuccessfullysensed) (Utilities|Struct|BreakAIStimulus Stimulus))
  (bind _returnvalue (AI|GetBlackboard 0))
  (if (Utilities|Name|Equal(Name) _tag "Noise")
    (AI|Components|Blackboard|SetValueasVector _returnvalue (Utilities|Name|MakeLiteralName "PlayerLastLocation") _stimuluslocation)
    (AI|Components|Blackboard|SetValueasBool _returnvalue (Utilities|Name|MakeLiteralName "PlayerSpotted") true)
    (Variables|Default|SetSpottedPlayer true)
    (else
      (AI|Components|Blackboard|SetValueasBool _returnvalue (Utilities|Name|MakeLiteralName "CanSeePlayer") _bsuccessfullysensed)
      (AI|Components|Blackboard|SetValueasBool _returnvalue (Utilities|Name|MakeLiteralName "PlayerSpotted") true)
      (Variables|Default|SetSpottedPlayer true)
      (AI|Components|Blackboard|SetValueasVector _returnvalue (Utilities|Name|MakeLiteralName "PlayerLastLocation") _stimuluslocation))))

(fn HostageSpotted
  (params (Stimulus :type AI%20Stimulus%20Structure) (Hostage :type BP%20Hostage%20Object%20Reference))
  (AI|Components|Blackboard|SetValueasBool (AI|GetBlackboard 0) (Utilities|Name|MakeLiteralName "CanSeeHostage") (.bSuccessfullySensed (Utilities|Struct|BreakAIStimulus Stimulus)))
  (Variables|Default|SetHostage Hostage))

(fn CheckLineOfFire
  (bind _returnvalue (Pawn|GetControlledPawn))
  (bind _outhit (Collision|SphereTraceByChannel (Transformation|GetSocketLocation (Variables|/Game/Characters/BP_Enemy.BP_Enemy_C|GetGlock (.AsBP%20Enemy (Utilities|Casting|CastToBP_Enemy _returnvalue))) "BulletSocket") (Transformation|GetActorLocation (Game|GetPlayerCharacter 0)) 3.0 "TraceTypeQuery2" false (Utilities|Array|MakeArray _returnvalue) "None"))
  (Utilities|Casting|CastToBP_Player (.HitActor (Collision|BreakHitResult _outhit))
    (:then
      (return true))
    (:CastFailed
      (return false))))

(fn HitPlayer
  (bind _returnvalue (Pawn|GetControlledPawn))
  (if (not (Variables|Default|GetIsHitting))
    (bind (_outhit _returnvalue_2) (Collision|LineTraceByChannel (Transformation|GetActorLocation _returnvalue) (Transformation|GetActorLocation (Game|GetPlayerCharacter 0)) "TraceTypeQuery2" false (Utilities|Array|MakeArray _returnvalue self) "None"))
    (if (and (<= (.distance _outhit) 1.5e+02) _returnvalue_2)
      (Utilities|Casting|CastToBP_Player (.hitactor _outhit))
      (Variables|Default|SetIsHitting true)
      (Utilities|Time|SetTimerbyFunctionName 0 "InvalidHit" 0.5))))

(fn InvalidHit
  (Variables|Default|SetIsHitting false))