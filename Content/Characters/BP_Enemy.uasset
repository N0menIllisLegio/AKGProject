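; BP_Enemy is the armed terrorist enemy character, built on a parent class with its own health, damage, name and hint text.
; StartShooting waits a second, then fires one Glock bullet from the muzzle socket with sound volume taken from the game instance.
; While on the ground, Tick zeroes the AI controller's yaw rotation.
; Death decrements the game mode's living-enemy count before running parent logic.
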(event Custom|StopShooting
  ;[1 1 1] Shooting
  (Variables|Default|SetIsShooting false))

(event Custom|StartShooting
  ;[1 1 1] Shooting
  (Variables|Default|SetIsShooting true)
  (Utilities|FlowControl|Delay 1.0)
  (CallFunction|ShootBullet))

(event EventBeginPlay
  ;[1 1 1] Init
  (|CallParentFunction)
  (bind _output_get (Variables|Default|SetFullHealth 1.5e+02))
  (Variables|Default|SetCurrentHealth _output_get)
  (Variables|Default|SetName "Террорист")
  (Variables|Default|SetDamage 1e+01)
  (Variables|/Game/HUDs/NpcHUD.NpcHUD_C|SetNpcGroup (Variables|Default|GetHUD) "NewEnumerator2"))

(event EventTick
  (params (DeltaSeconds :type Float%20%28single-precision%29))
  ;[1 1 1] StopRotation
  (|CallParentFunction DeltaSeconds)
  (if (AI|Components|NavMovement|IsMovingonGround (Variables|Character|GetCharacterMovement))
    (bind _asbp_enemy_ai (Utilities|Casting|CastToBP_EnemyAI (Pawn|GetController)))
    (Variables|/Game/Characters/AI/Enemy/BP_EnemyAI.BP_EnemyAI_C|SetRotationYaw _asbp_enemy_ai 0.0)))

(event EventDie
  ;[1 1 1] Death
  (bind _asbp_base_game_mode (Utilities|Casting|CastToBP_BaseGameMode (Game|GetGameMode))
    (:then
      (Math|Integer|DecrementInt (Variables|/Game/GameModes/BP_BaseGameMode.BP_BaseGameMode_C|GetEnemiesAlive _asbp_base_game_mode)
        (:%20%20
          _)))
    (:CastFailed
      _))
  (|CallParentFunction))

(fn ConstructionScript
  (|CallParentFunction))

(fn ShootBullet
  (bind _glock (Variables|Default|GetGlock))
  (bind _returnvalue (Transformation|GetSocketLocation _glock "BulletSocket"))
  (Audio|PlaySoundatLocation "/Game/Sounds/Weapons/Glock/Glock18-2_Cue.Glock18-2_Cue" _returnvalue "0, 0, 0" (Variables|/Game/BP_GameInstance.BP_GameInstance_C|GetSounds (.AsBP%20Game%20Instance (Utilities|Casting|CastToBP_GameInstance (Game|GetGameInstance)))) 1.0 0.0 0 0 0)
  (Game|SpawnActorfromClass "/Game/Characters/Assets/BP_Bullet_Glock.BP_Bullet_Glock_C" (Math|Transform|MakeTransform _returnvalue (Math|Rotator|CombineRotators (Transformation|GetSocketRotation _glock "BulletSocket") "0, 0, 0")) "AdjustIfPossibleButAlwaysSpawn" 0 self))

(fn GetHint
  (return true "Террорист" "В миссиях на устранение террористов, необходимо убить их всех." "Нажмите ЛКМ, чтобы выстрелить. 
Нажмите E, чтобы ударить."))