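; BP_Hostage is a hostage NPC that follows the player when interacted with, to be brought to an APC in rescue missions.
; It extends a parent NPC class, setting health, name, HUD group and hint text.
; Interact focuses BP_HostageAI on the user, plays a voice cue and sets follow flags.
; Resque and Die update the game mode's hostage counters; Resque also destroys the actor and notifies the HUD.
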(event EventBeginPlay
  ;[1 1 1] Add npc group
  (|CallParentFunction)
  (bind _output_get (Variables|Default|SetFullHealth 1e+02))
  (Variables|Default|SetCurrentHealth _output_get)
  (Variables|Default|SetName "Заложник")
  (Variables|/Game/HUDs/NpcHUD.NpcHUD_C|SetNpcGroup (Variables|Default|GetHUD) "NewEnumerator3"))

(event EventTick
  (params (DeltaSeconds :type Float%20%28single-precision%29))
  (|CallParentFunction DeltaSeconds) ; This node is disabled and will not be called.\nDrag off pins to build functionality.
)

(event EventDie
  (bind _asbp_base_game_mode (Utilities|Casting|CastToBP_BaseGameMode (Game|GetGameMode))
    (:then
      (Math|Integer|DecrementInt (Variables|/Game/GameModes/BP_BaseGameMode.BP_BaseGameMode_C|GetHostagesAlive _asbp_base_game_mode)
        (:%20%20
          _)))
    (:CastFailed
      _))
  (|CallParentFunction))

(fn ConstructionScript
  (|CallParentFunction))

(fn Resque
  (bind _asbp_base_game_mode (Utilities|Casting|CastToBP_BaseGameMode (Game|GetGameMode)))
  (Math|Integer|IncrementInt (Variables|/Game/GameModes/BP_BaseGameMode.BP_BaseGameMode_C|GetResquedHostages _asbp_base_game_mode)
    (:%20%20
      (Actor|DestroyActor)
      (Default|HostageResqued (Variables|/Game/GameModes/BP_BaseGameMode.BP_BaseGameMode_C|GetGameHUDReference _asbp_base_game_mode)))))

(fn Interact
  (params (User :type BP%20Base%20Character%20Object%20Reference))
  (bind _asbp_hostage_ai (Utilities|Casting|CastToBP_HostageAI (Pawn|GetController)))
  (Default|Focusing _asbp_hostage_ai User)
  (Audio|PlaySoundatLocation "/Game/Sounds/Hostage/hos4_Cue.hos4_Cue" (Transformation|GetActorLocation (Game|GetPlayerCharacter 0)) "0, 0, 0" (Variables|/Game/BP_GameInstance.BP_GameInstance_C|GetSounds (.AsBP%20Game%20Instance (Utilities|Casting|CastToBP_GameInstance (Game|GetGameInstance)))) 1.0 0.0 0 0 0)
  (Variables|Default|SetIsFollowingPlayer true)
  (Variables|Default|SetOnStartingPosition false)
  (bind _completed (|CallParentFunction 0))
  (return _completed))

(fn GetHint
  (return true "Заложник" "Заложник, в миссиях по освобождениию заложников, надо привести к БТРу." "Нажмите F, чтобы он последовал за вами."))