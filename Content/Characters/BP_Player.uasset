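; Player character with an M4A1, managing health, ammo, up to two grenades, a silencer and night-vision goggles.
; Construction loads health and ammo from BP_GameInstance, and death clears PlayerAlive on BP_BaseGameMode.
; Each tick a trace from the muzzle socket sets the laser beam's endpoint at the hit or maximum range.
; Functions handle reloading and pickups, sync grenade HUD icons, reposition the goggles, and toggle silencer mesh and shot volume.
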(event EventTick
  (params (DeltaSeconds :type Float%20%28single-precision%29))
  ;[1 1 1] Laser
  (bind (_hitresult _ishitted) (Utilities|LaserDistance (Variables|Default|GetLaser_Distance))
    (:Out
      (CallFunction|DrawLaser _ishitted (.ImpactPoint (Collision|BreakHitResult _hitresult)) (Variables|Default|GetLaser_Distance)))))

(event EventBeginPlay
  (bind _nvg (Variables|Default|GetNVG))
  (Variables|Default|SetNVPos (Variables|/Script/Engine.SceneComponent|GetRelativeLocation _nvg))
  (Variables|Default|SetNVRot (Variables|/Script/Engine.SceneComponent|GetRelativeRotation _nvg)))

(event EventDie
  ;[1 1 1] Death
  (bind _asbp_base_game_mode (Utilities|Casting|CastToBP_BaseGameMode (Game|GetGameMode)))
  (Variables|/Game/GameModes/BP_BaseGameMode.BP_BaseGameMode_C|SetPlayerAlive _asbp_base_game_mode false))

(fn ConstructionScript
  (bind _asbp_game_instance (Utilities|Casting|CastToBP_GameInstance (Game|GetGameInstance)))
  (Variables|Default|SetCurrentHealth (Variables|/Game/BP_GameInstance.BP_GameInstance_C|GetCharacterHealth _asbp_game_instance))
  (Variables|Default|SetFullHealth 2e+02)
  (Variables|Default|SetNotLoadedAmmo (Variables|/Game/BP_GameInstance.BP_GameInstance_C|GetNotLoadedAmmo _asbp_game_instance))
  (Variables|Default|SetMaxNotLoadedAmmo 120)
  (Variables|Default|SetLoadedAmmo (Variables|/Game/BP_GameInstance.BP_GameInstance_C|GetLoadedAmmo _asbp_game_instance))
  (Variables|Default|SetMaxLoadedAmmo 30)
  (Variables|Default|SetLaser_Distance 5e+03)
  (Variables|Default|SetName "Player")
  (Variables|Default|SetThrustDamage 1e+01))

(fn TraceLaser
  (bind _sm_m4a1 (Variables|Default|GetSM_M4A1))
  (bind _returnvalue (Transformation|GetSocketLocation _sm_m4a1 "ShootSocket"))
  (Collision|LineTraceByChannel _returnvalue (+ _returnvalue (* (Math|Vector|GetForwardVector (Transformation|GetSocketRotation _sm_m4a1 "ShootSocket")) 5e+03)) "TraceTypeQuery1" false (Utilities|Array|MakeArray self) "ForOneFrame"))

(fn DrawLaser
  (params (IsHitted :type Boolean) (ImpactLocation :type Vector) (LaserDistance :type Float%20%28single-precision%29))
  (bind _sm_m4a1 (Variables|Default|GetSM_M4A1))
  (bind _returnvalue (Transformation|GetSocketLocation _sm_m4a1 "ShootSocket"))
  (if IsHitted
    (LocalVariables|SetTargetPoint ImpactLocation)
    (else
      (LocalVariables|SetTargetPoint (+ _returnvalue (* (Math|Vector|GetForwardVector (Transformation|GetSocketRotation _sm_m4a1 "ShootSocket")) LaserDistance)))))
  (Class|ParticleSystemComponent|SetBeamSourcePoint (Variables|Default|GetLaser) 0 _returnvalue)
  (Class|ParticleSystemComponent|SetBeamTargetPoint (Variables|Default|GetLaser) 0 (LocalVariables|GetTargetPoint)))

(fn Reload
  (if (<= (- (Variables|Default|GetMaxLoadedAmmo) (Variables|Default|GetLoadedAmmo)) (Variables|Default|GetNotLoadedAmmo))
    (Variables|Default|SetNotLoadedAmmo (- (Variables|Default|GetNotLoadedAmmo) (- (Variables|Default|GetMaxLoadedAmmo) (Variables|Default|GetLoadedAmmo))))
    (Variables|Default|SetLoadedAmmo (Variables|Default|GetMaxLoadedAmmo))
    (else
      (Variables|Default|SetLoadedAmmo (+ (Variables|Default|GetLoadedAmmo) (Variables|Default|GetNotLoadedAmmo)))
      (Variables|Default|SetNotLoadedAmmo 0))))

(fn PickAmmo
  (params (Ammo :type Integer))
  (if (== (Variables|Default|GetMaxNotLoadedAmmo) (Variables|Default|GetNotLoadedAmmo))
    (return false)
    (else
      (Variables|Default|SetNotLoadedAmmo (Math|Integer|Min(Integer) (+ Ammo (Variables|Default|GetNotLoadedAmmo)) (Variables|Default|GetMaxNotLoadedAmmo)))
      (return true))))

(fn OffNVG
  (bind _nvg (Variables|Default|GetNVG))
  (Transformation|SetRelativeLocation _nvg (Variables|Default|GetNVPos) false false)
  (Transformation|SetRelativeRotation _nvg (Variables|Default|GetNVRot) false false))

(fn OnNVG
  (bind _nvg (Variables|Default|GetNVG))
  (Transformation|SetRelativeLocation _nvg "-0.473016,10.501570,5.954227" false false)
  (Transformation|SetRelativeRotation _nvg "95.000244,90.002747,0.000153" false false))

(fn PickGrenade
  (bind _returnvalue (Game|GetGameMode))
  (if (< (Variables|Default|GetGrenades) 2)
    (bind _result (Math|Integer|IncrementInt (Variables|Default|GetGrenades))
      (:%20%20
        (switch int _result
          (:1
            (bind _asbp_base_game_mode (Utilities|Casting|CastToBP_BaseGameMode _returnvalue))
            (Widget|SetVisibility (Variables|/Game/HUDs/PlayerHUD.PlayerHUD_C|GetGrenadeImg_1 (Variables|/Game/GameModes/BP_BaseGameMode.BP_BaseGameMode_C|GetGameHUDReference _asbp_base_game_mode)) "Visible"))
          (:2
            (bind _asbp_base_game_mode_2 (Utilities|Casting|CastToBP_BaseGameMode _returnvalue))
            (Widget|SetVisibility (Variables|/Game/HUDs/PlayerHUD.PlayerHUD_C|GetGrenadeImg_2 (Variables|/Game/GameModes/BP_BaseGameMode.BP_BaseGameMode_C|GetGameHUDReference _asbp_base_game_mode_2)) "Visible")))
        (return true)))
    (else
      (return false))))

(fn ThrowGrenade
  (bind _returnvalue (Game|GetGameMode))
  (bind _result (Math|Integer|DecrementInt (Variables|Default|GetGrenades))
    (:%20%20
      (switch int _result
        (:0
          (bind _asbp_base_game_mode (Utilities|Casting|CastToBP_BaseGameMode _returnvalue))
          (Widget|SetVisibility (Variables|/Game/HUDs/PlayerHUD.PlayerHUD_C|GetGrenadeImg_1 (Variables|/Game/GameModes/BP_BaseGameMode.BP_BaseGameMode_C|GetGameHUDReference _asbp_base_game_mode)) "Hidden"))
        (:1
          (bind _asbp_base_game_mode_2 (Utilities|Casting|CastToBP_BaseGameMode _returnvalue))
          (Widget|SetVisibility (Variables|/Game/HUDs/PlayerHUD.PlayerHUD_C|GetGrenadeImg_2 (Variables|/Game/GameModes/BP_BaseGameMode.BP_BaseGameMode_C|GetGameHUDReference _asbp_base_game_mode_2)) "Hidden"))))))

(fn OnSilencer
  (if (Variables|Default|GetSilencer)
    (Rendering|SetVisibility (Variables|Default|GetSM_M4A1_Silencer) true false)
    (Variables|Default|SetShootVolume 0.25)))

(fn OffSilencer
  (if (Variables|Default|GetSilencer)
    (Rendering|SetVisibility (Variables|Default|GetSM_M4A1_Silencer) false false)
    (Variables|Default|SetShootVolume 1.0)))