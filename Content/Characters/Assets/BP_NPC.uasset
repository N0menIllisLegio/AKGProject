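; NPC character with an overhead HUD widget, automatic door opening and stubbed interaction.
; Each tick a camera-channel trace from the chest shows the widget only when the player is in range and unobstructed.
; Overlapping a BP_Door starts a looping timer that opens it whenever closed.
; Focus uses a retriggerable delay to toggle a light and HUD hint; Thrust applies damage, while Interact and GetHint return empty defaults.
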(event Custom|Checking
  (bind _door (Variables|Default|GetDoor))
  ;[1 1 1] OpenDoors
  (Utilities|IsValid _door
    (:Is%20Valid
      (if (Variables|/Game/Actors/BP_Door.BP_Door_C|GetIsDoorClosed _door)
        (Default|Interact _door self)))))

(event EventBeginPlay
  ;[1 1 1] INCOMPLEAT
  (|CallParentFunction)
  (bind _asnpc_hud (Utilities|Casting|CastToNpcHUD (UserInterface|GetUserWidgetObject (Variables|Default|GetNPCUI))))
  (bind _output_get (Variables|Default|SetHUD _asnpc_hud))
  (Variables|/Game/HUDs/NpcHUD.NpcHUD_C|SetNPC _output_get self)
  (Variables|/Game/HUDs/NpcHUD.NpcHUD_C|SetNpcGroup _output_get "NewEnumerator0"))

(event Collision|EventActorBeginOverlap
  (params (OtherActor :type Actor%20Object%20Reference))
  ;[1 1 1] OpenDoors
  (bind _asbp_door (Utilities|Casting|CastToBP_Door OtherActor))
  (Variables|Default|SetDoor _asbp_door)
  (bind _returnvalue (Utilities|Time|SetTimerbyEvent (delegate Custom|Checking) 0.2 true)))

(event Collision|EventActorEndOverlap
  (params (OtherActor :type Actor%20Object%20Reference))
  ;[1 1 1] OpenDoors
  (Utilities|Casting|CastToBP_Door OtherActor)
  (Variables|Default|SetDoor 0)
  (Utilities|Time|ClearandInvalidateTimerbyHandle (stale Collision|EventActorBeginOverlap _returnvalue)))

(event EventOnFocus
  (CallFunction|OnBeginFocus)
  (Utilities|FlowControl|RetriggerableDelay 0.1)
  (CallFunction|OnEndFocus))

(event EventTick
  (params (DeltaSeconds :type Float%20%28single-precision%29))
  (|CallParentFunction DeltaSeconds)
  (Utilities|IsValid (Game|GetPlayerCharacter 0)
    (:Is%20Valid
      (CallFunction|WidgetVisibilitytoPlayer))))

(fn ConstructionScript
  (|CallParentFunction))

(fn WidgetVisibilitytoPlayer
  (bind _npcui (Variables|Default|GetNPCUI))
  (bind _location (CallFunction|GetChestLocation))
  (bind _outhit (Collision|LineTraceByChannel _location (Transformation|GetActorLocation (Game|GetPlayerCharacter 0)) "TraceTypeQuery2" false 0 "None"))
  (Utilities|Casting|CastToBP_Player (.HitActor (Collision|BreakHitResult _outhit))
    (:then
      (Rendering|SetVisibility _npcui (<= (.Distance (Collision|BreakHitResult _outhit)) 1.2e+03) false))
    (:CastFailed
      (Rendering|SetVisibility _npcui false false))))

(fn Check
  (return true))

(fn GetHint
  (return false "" "" ""))

(fn Interact
  (params (User :type BP%20Base%20Character%20Object%20Reference))
  (return false))

(fn OnBeginFocus
  (Rendering|SetVisibility (Variables|Default|GetPointLight) true false)
  (bind _asbp_base_game_mode (Utilities|Casting|CastToBP_BaseGameMode (Game|GetGameMode)))
  (Default|DisplayHint (Variables|/Game/GameModes/BP_BaseGameMode.BP_BaseGameMode_C|GetGameHUDReference _asbp_base_game_mode) self)
  (return true))

(fn OnEndFocus
  (Rendering|SetVisibility (Variables|Default|GetPointLight) false false)
  (bind _asbp_base_game_mode (Utilities|Casting|CastToBP_BaseGameMode (Game|GetGameMode)))
  (Default|HideHint (Variables|/Game/GameModes/BP_BaseGameMode.BP_BaseGameMode_C|GetGameHUDReference _asbp_base_game_mode))
  (return true))

(fn Thrust
  (params (Direction :type Vector :default "0, 0, 0") (Power :type Float%20%28single-precision%29) (Damage :type Float%20%28single-precision%29) (User :type BP%20Base%20Character%20Object%20Reference))
  (CallFunction|TakeDamage Damage)
  (return true))