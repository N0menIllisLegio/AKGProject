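; Base bullet actor that damages the character it hits and expires after a one-second lifespan.
; On spawn, its sphere ignores the instigator while moving so the bullet does not collide with its shooter.
; Only the first hit is processed: if it is a BP_BaseCharacter, the bullet reports an AI damage-sense event, then calls TakeDamage on it.
; Damage comes from GetBulletDamage, which returns the initial bullet damage value.
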(event EventBeginPlay
  (Collision|IgnoreActorwhenMoving (Variables|Default|GetSphere) (Game|GetInstigator) true)
  (Actor|SetLifeSpan 1.0))

(event Collision|EventHit
  (params (MyComp :type Primitive%20Component%20Object%20Reference) (Other :type Actor%20Object%20Reference) (OtherComp :type Primitive%20Component%20Object%20Reference) (bSelfMoved :type Boolean) (HitLocation :type Vector :default "0, 0, 0") (HitNormal :type Vector :default "0, 0, 0") (NormalImpulse :type Vector :default "0, 0, 0") (Hit :type Hit%20Result%20Structure%20%28by%20ref%29))
  (bind _hitactor (Collision|BreakHitResult Hit))
  (Utilities|FlowControl|DoOnce false
    (:Completed
      (bind _asbp_base_character (Utilities|Casting|CastToBP_BaseCharacter _hitactor))
      (bind _damage (CallFunction|GetBulletDamage))
      (Class|AISenseDamage|ReportDamageEvent _hitactor (Game|GetInstigator) _damage (Transformation|GetActorLocation))
      (Default|TakeDamage _asbp_base_character _damage))))

(fn ConstructionScript)

(fn GetBulletDamage
  (return (Variables|Default|GetInitBulletDamage)))