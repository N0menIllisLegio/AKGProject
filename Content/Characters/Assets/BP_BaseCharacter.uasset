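; Base character Blueprint that provides health, damage, healing and death logic.
; TakeDamage floors CurrentHealth at zero and calls Die, which plays a death sound scaled by the game instance's Sounds value, then destroys the actor.
; Heal caps health at FullHealth and returns false when it is already full.
; GetChestLocation returns the mesh's Spine2 socket position.
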(fn ConstructionScript)

(fn Die
  (Audio|PlaySoundatLocation "/Game/Sounds/Hurt/death6_Cue.death6_Cue" (Transformation|GetActorLocation) "0, 0, 0" (Variables|/Game/BP_GameInstance.BP_GameInstance_C|GetSounds (.AsBP%20Game%20Instance (Utilities|Casting|CastToBP_GameInstance (Game|GetGameInstance)))) 1.0 0.0 0 0 0)
  (Actor|DestroyActor))

(fn Heal
  (params (HP :type Float%20%28single-precision%29))
  (if (== (Variables|Default|GetCurrentHealth) (Variables|Default|GetFullHealth))
    (return false)
    (else
      (Variables|Default|SetCurrentHealth (Math|Float|Min(Float) (+ HP (Variables|Default|GetCurrentHealth)) (Variables|Default|GetFullHealth)))
      (return true))))

(fn TakeDamage
  (params (Damage :type Float%20%28single-precision%29))
  (bind _output_get (Variables|Default|SetCurrentHealth (Math|Float|Max(Float) (- (Variables|Default|GetCurrentHealth) Damage) 0.0)))
  (if (<= _output_get 0.0)
    (CallFunction|Die)))

(fn GetChestLocation
  (return (Transformation|GetSocketLocation (Variables|Character|GetMesh) "Spine2")))