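; BP_MenuPlayerController is a player controller, named for the menu, that provides first-person-style look input without a visible cursor.
; On BeginPlay it hides the mouse cursor, sets game-only input, then fetches player pawn 0 and possesses it.
; Turn and LookUp axis events feed yaw and pitch input to that pawn at half strength.
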(event EventBeginPlay
  (bind _self self)
  (Variables|/Script/Engine.PlayerController|SetbShowMouseCursor _self false)
  (Input|SetInputModeGameOnly _self)
  (bind _output_get (Variables|Default|SetMenuPlayer (Game|Player|GetPlayerPawn 0)))
  (Pawn|Possess _output_get))

(event EventTick
  (params (DeltaSeconds :type Float%20%28single-precision%29)))

(event Input|AxisEvents|InputAxisTurn
  (params (AxisValue :type Float%20%28single-precision%29))
  ;[1 1 1] Camera Movement
  (Pawn|Input|AddControllerYawInput (Variables|Default|GetMenuPlayer) (/ AxisValue 2.0)))

(event Input|AxisEvents|InputAxisLookUp
  (params (AxisValue :type Float%20%28single-precision%29))
  ;[1 1 1] Camera Movement
  (Pawn|Input|AddControllerPitchInput (Variables|Default|GetMenuPlayer) (/ AxisValue 2.0)))

(fn ConstructionScript)