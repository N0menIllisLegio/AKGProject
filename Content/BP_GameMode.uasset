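; Game mode that sets the win and lose rules for a timed level where the player must eliminate all enemies without killing civilians.
; BeginPlay sets the time limit, counts placed BP_Enemy actors, resets the alive flags and shows the player HUD.
; Tick polls those values, calling Victory when no enemies remain or Defeat with a cause for death, civilian kill or timeout.
; Both outcomes pause the game and show their end screen with cursor and UI-only input.
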(event EventBeginPlay
  ;[1 1 1] Initialization
  (Variables|Default|SetTimeLimit 1.8e+02)
  (bind _outactors (Actor|GetAllActorsOfClass "/Game/Pawns/BP_Enemy.BP_Enemy_C"))
  (bind _output_get (Variables|Default|SetEnemiesCount (Utilities|Array|Length _outactors)))
  (Variables|Default|SetTotalEnemies _output_get)
  (Variables|Default|SetPlayerAlive true)
  (Variables|Default|SetAllCiviliansAlive true)
  (bind _returnvalue (UserInterface|CreateWidget "/Game/HUDs/PlayerHUD.PlayerHUD_C"))
  (bind _output_get_2 (Variables|Default|SetGameHUDReference _returnvalue))
  (UserInterface|Viewport|AddtoViewport _output_get_2 0))

(event EventTick
  (params (DeltaSeconds :type Float%20%28single-precision%29))
  ;[1 1 1] Check rules
  (if (Variables|Default|GetPlayerAlive)
    (if (Variables|Default|GetAllCiviliansAlive)
      (if (> (Variables|Default|GetTimeLimit) (Utilities|Time|GetGameTimeinSeconds))
        (if (not (> (Variables|Default|GetEnemiesCount) 0))
          (CallFunction|Victory))
        (else
          (CallFunction|Defeat "You areout of time!")))
      (else
        (CallFunction|Defeat "You Killed Civilian. Monster!")))
    (else
      (CallFunction|Defeat "You Died"))))

(fn ConstructionScript)

(fn Victory
  (bind _returnvalue (Game|GetPlayerController 0))
  (Game|SetGamePaused true)
  (bind _returnvalue_2 (UserInterface|CreateWidget "/Game/HUDs/VictoryHUD.VictoryHUD_C"))
  (UserInterface|Viewport|AddtoViewport _returnvalue_2 0)
  (Variables|/Script/Engine.PlayerController|SetbShowMouseCursor _returnvalue true)
  (Input|SetInputModeUIOnly _returnvalue _returnvalue_2 "DoNotLock"))

(fn Defeat
  (params (CauseOfDefeat :type String))
  (bind _returnvalue (Game|GetPlayerController 0))
  (Variables|Default|SetCauseOfDefeat CauseOfDefeat)
  (Game|SetGamePaused true)
  (bind _returnvalue_2 (UserInterface|CreateWidget "/Game/HUDs/DefeatHUD.DefeatHUD_C"))
  (UserInterface|Viewport|AddtoViewport _returnvalue_2 0)
  (Variables|/Script/Engine.PlayerController|SetbShowMouseCursor _returnvalue true)
  (Input|SetInputModeUIOnly _returnvalue _returnvalue_2 "DoNotLock"))