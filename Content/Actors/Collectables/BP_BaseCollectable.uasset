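; Base collectable actor that spins and bobs in place until it is used or hit.
; Tick yaws it at a steady rate and moves it along local Z, with ChangeDirection flipping the travel sign based on distance to its Owner.
; The bob therefore relies on an Owner actor as its reference point.
; Interact and Thrust both just destroy the actor and return true, ignoring their inputs.
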(event EventBeginPlay
  (Variables|Default|SetDirection 1e+01))

(event Collision|EventActorBeginOverlap
  (params (OtherActor :type Actor%20Object%20Reference)))

(event EventTick
  (params (DeltaSeconds :type Float%20%28single-precision%29))
  ;[1 1 1] Collectable animation
  (Transformation|AddActorLocalRotation (Math|Rotator|MakeRotator 0.0 0.0 (* DeltaSeconds 2e+01)) false false)
  (CallFunction|ChangeDirection)
  (Transformation|AddActorLocalOffset (Math|Vector|MakeVector 0.0 0.0 (* DeltaSeconds (Variables|Default|GetDirection))) false false))

(fn ConstructionScript)

(fn ChangeDirection
  (bind _returnvalue (Components|GetOwner))
  (bind _returnvalue_2 (Transformation|GetDistanceTo _returnvalue))
  (if (> _returnvalue_2 1.2e+02)
    (Variables|Default|SetDirection -1e+01)
    (elif (< _returnvalue_2 65.0)
      (Variables|Default|SetDirection 1e+01)))
  (return))

(fn Interact
  (params (User :type BP%20Player%20Object%20Reference))
  (Actor|DestroyActor)
  (return true))

(fn Thrust
  (params (Direction :type Vector :default "0, 0, 0") (Power :type Float%20%28single-precision%29) (Damage :type Float%20%28single-precision%29))
  (Actor|DestroyActor)
  (return true))