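; BP_Ammo is a collectable ammo pickup that holds a fixed amount of rounds, set on BeginPlay.
; On Interact it offers them to BP_Player through PickAmmo and runs the parent interaction only if they are accepted.
; GetHint extends the parent hint with a Russian name and description, which says pickup fails when reserve ammo is full.
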(event EventBeginPlay
  (|CallParentFunction)
  (Variables|Default|SetAmmo 10))

(event Collision|EventActorBeginOverlap
  (params (OtherActor :type Actor%20Object%20Reference)))

(event EventTick
  (params (DeltaSeconds :type Float%20%28single-precision%29))
  (|CallParentFunction DeltaSeconds))

(fn ConstructionScript)

(fn Interact
  (params (User :type BP%20Base%20Character%20Object%20Reference))
  (bind _asbp_player (Utilities|Casting|CastToBP_Player User))
  (bind _picked (Default|PickAmmo _asbp_player (Variables|Default|GetAmmo)))
  (if _picked
    (bind _completed (|CallParentFunction _asbp_player))
    (return _completed)))

(fn GetHint
  (bind (_complete _hintname _hintdescrption _hintinteraction) (|CallParentFunction))
  (return _complete "Патроны" "Увеличивают количество не заряженных в магазин патронов. Если не заряженных патронов максимум, то патроны подняты не будут." _hintinteraction))