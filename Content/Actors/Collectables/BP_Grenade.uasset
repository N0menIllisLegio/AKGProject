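; BP_Grenade is a collectable grenade that players can pick up, throw or break.
; Interact calls PickGrenade on BP_Player and destroys the actor on success, while GetHint supplies Russian name, description and control text.
; Throw starts a timer to Explode, which spawns BP_Explosion at the mesh location and destroys the grenade.
; Thrust destroys it without exploding, as its Explode call is disconnected.
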(fn ConstructionScript
  (|CallParentFunction))

(fn Throw
  (Utilities|Time|SetTimerbyFunctionName 0 "Explode" (Variables|Default|GetExplodeTime)))

(fn Explode
  (Game|SpawnActorfromClass "/Game/Actors/BP_Explosion.BP_Explosion_C" (Math|Transform|MakeTransform (Transformation|GetWorldLocation (Variables|Default|GetStaticMesh)) "0, 0, 0" "1,1,1") "Undefined" 0 0)
  (Actor|DestroyActor))

(fn Check
  (return true))

(fn Thrust
  (params (Direction :type Vector :default "0, 0, 0") (Power :type Float%20%28single-precision%29) (Damage :type Float%20%28single-precision%29) (User :type BP%20Base%20Character%20Object%20Reference))
  (Actor|DestroyActor)
  (return true))

(fn Interact
  (params (User :type BP%20Base%20Character%20Object%20Reference))
  (bind _asbp_player (Utilities|Casting|CastToBP_Player User))
  (bind _picked (Default|PickGrenade _asbp_player))
  (if _picked
    (Actor|DestroyActor)
    (return true)))

(fn GetHint
  (bind _complete (|CallParentFunction))
  (return _complete "Граната" "Взрывается. Максимальное количество, которое можно носить - 2 штуки." "Нажмите F, чтобы поднять гранату. 
Нажмите E, чтобы сломать гранату. 
Нажмите G, чтобы бросить гранату."))