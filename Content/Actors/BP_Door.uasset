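; BP_Door is a door actor that can be opened and closed through Interact or knocked down by Thrust.
; OpenCloseDoor timeline drives the mesh's world yaw, playing or reversing based on IsClosed.
; Thrust plays KnockOut to pitch a closed door by the sign of Direction.X, setting IsKnockedOut to block further actions.
; The IsClosed graph shows only an unused near-zero yaw comparison.
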(event EventBeginPlay
  (Variables|Default|SetIsKnockedOut false))

(event EventThrust
  (params (Direction :type Vector :default "0, 0, 0") (Power :type Float%20%28single-precision%29) (Damage :type Float%20%28single-precision%29))
  (if (and (not (Variables|Default|GetIsKnockedOut)) (Utilities|IsClosed))
    (Variables|Default|SetIsKnockedOut true)
    (bind _rotation (Timeline|KnockOut Play)
      (:Update
        (Transformation|SetWorldRotation (Variables|Default|GetStaticMesh) (Math|Rotator|MakeRotator 0.0 (* _rotation (* (Math|Float|Sign(Float) (.X (Math|Vector|BreakVector Direction))) -1.0)) 0.0) false false)))))

(event EventInteract
  (params (User :type BP%20Player%20Object%20Reference))
  (if (not (Variables|Default|GetIsKnockedOut))
    (if (Utilities|IsClosed)
      (bind _rotation (Timeline|OpenCloseDoor Play)
        (:Update
          (Transformation|SetWorldRotation (Variables|Default|GetStaticMesh) (Math|Rotator|MakeRotator 0.0 0.0 _rotation) false false)))
      (else
        (Timeline|OpenCloseDoor Reverse)))))

(fn ConstructionScript)