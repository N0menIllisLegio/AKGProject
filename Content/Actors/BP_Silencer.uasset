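; BP_Silencer is a world pickup for the M16 rifle silencer.
; Interact sets the Silencer flag on BP_Player and destroys the actor, while GetHint supplies Russian name, description and key-prompt text.
; Focus shows a point light and a HUD hint through BP_BaseGameMode's HUD reference.
; OnFocus restarts a short RetriggerableDelay on each call, so light and hint clear automatically once focus calls stop.
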(event EventOnFocus
  (CallFunction|OnBeginFocus)
  (Utilities|FlowControl|RetriggerableDelay 0.1)
  (CallFunction|OnEndFocus))

(fn ConstructionScript)

(fn Check
  (return true))

(fn GetHint
  (return true "Глушитель" "Глушитель для винтовки M16. Глушит звуки выстрелов." "Нажмите F, чтобы поднять глушитель. 
Нажмите T, чтобы прикрутить\\снять глушитель."))

(fn Interact
  (params (User :type BP%20Base%20Character%20Object%20Reference))
  (bind _asbp_player (Utilities|Casting|CastToBP_Player User))
  (Variables|/Game/Characters/BP_Player.BP_Player_C|SetSilencer _asbp_player true)
  (Actor|DestroyActor)
  (return true))

(fn OnBeginFocus
  (Rendering|SetVisibility (Variables|Default|GetPointLight) true false)
  (bind _asbp_base_game_mode (Utilities|Casting|CastToBP_BaseGameMode (Game|GetGameMode)))
  (Default|DisplayHint (Variables|/Game/GameModes/BP_BaseGameMode.BP_BaseGameMode_C|GetGameHUDReference _asbp_base_game_mode) self)
  (return true))

(fn OnEndFocus
  (Rendering|SetVisibility (Variables|Default|GetPointLight) false false)
  (bind _asbp_base_game_mode (Utilities|Casting|CastToBP_BaseGameMode (Game|GetGameMode)))
  (Default|HideHint (Variables|/Game/GameModes/BP_BaseGameMode.BP_BaseGameMode_C|GetGameHUDReference _asbp_base_game_mode))
  (return true))

(fn Thrust
  (params (Direction :type Vector :default "0, 0, 0") (Power :type Float%20%28single-precision%29) (Damage :type Float%20%28single-precision%29) (User :type BP%20Base%20Character%20Object%20Reference))
  (return false))