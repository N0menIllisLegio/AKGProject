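; BP_Bomb is a defusable mission bomb that explodes when its countdown ends or it is thrust, except in LevelTutorial.
; Explosion plays sound and effects, cancels defusing, then flags the loss in BP_BombGameMode after a delay.
; Defusing uses a looping timer whose interval sets the speed; completion flags the bomb diffused, while interruption resets progress.
; Focus uses a retriggerable delay to show a light and HUD hint briefly.
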(event EventBeginPlay
  (Utilities|FlowControl|Sequence
    (:then_0
      (bind _output_get (Variables|Default|SetTimer 1.8e+02))
      (Utilities|Time|SetTimerbyFunctionName 0 "Explode" _output_get))
    (:then_1
      (Variables|Default|SetTotalDiffusingTimer 1e+01)
      (Variables|Default|SetCurrentDiffusingTimer 0.0))))

(event EventOnFocus
  (CallFunction|OnBeginFocus)
  (Utilities|FlowControl|RetriggerableDelay 0.1)
  (CallFunction|OnEndFocus))

(fn ConstructionScript)

(fn Explode
  (bind _returnvalue (Transformation|GetActorLocation))
  (bind _returnvalue_2 (Game|GetCurrentLevelName true))
  (if (not (Utilities|Enum|Equal(Enum) _returnvalue_2 "LevelTutorial"))
    (Audio|PlaySoundatLocation "/Game/Sounds/Weapons/C4/c4_explode_Cue.c4_explode_Cue" _returnvalue "0, 0, 0" (Variables|/Game/BP_GameInstance.BP_GameInstance_C|GetSounds (.AsBP%20Game%20Instance (Utilities|Casting|CastToBP_GameInstance (Game|GetGameInstance)))) 1.0 0.0 0 0 0)
    (Effects|SpawnEmitteratLocation "/Game/Particles/P_Explosion.P_Explosion" _returnvalue "0, 0, 0" "10.000000,10.000000,10.000000")
    (Utilities|Time|SetTimerbyFunctionName 0 "Lose" 2.0)
    (Variables|Default|SetExploded true)
    (CallFunction|EndDiffusing)))

(fn StartDiffusing
  (params (DiffusingSpeed :type Float%20%28single-precision%29))
  (if (not (Variables|Default|GetExploded))
    (bind _returnvalue (Utilities|Time|SetTimerbyFunctionName 0 "Diffuse" DiffusingSpeed true))
    (Variables|Default|SetDiffuseTimer _returnvalue)
    (Variables|Default|SetDiffusing true)))

(fn EndDiffusing
  (bind _diffusetimer (Variables|Default|GetDiffuseTimer))
  (if (Utilities|Time|IsValidTimerHandle _diffusetimer)
    (Utilities|Time|ClearandInvalidateTimerbyHandle _diffusetimer))
  (Variables|Default|SetDiffusing false)
  (Variables|Default|SetCurrentDiffusingTimer 0.0)
  (bind _asbp_player_controller (Utilities|Casting|CastToBP_PlayerController (Game|GetPlayerController 0)))
  (Variables|/Game/Characters/BP_PlayerController.BP_PlayerController_C|SetDiffusingBomb _asbp_player_controller 0)
  (Default|EndDiffusing _asbp_player_controller))

(fn Diffuse
  (bind _output_get (Variables|Default|SetCurrentDiffusingTimer (+ (Variables|Default|GetCurrentDiffusingTimer) 0.1)))
  (if (>= _output_get (Variables|Default|GetTotalDiffusingTimer))
    (CallFunction|EndDiffusing)
    (bind _asbp_bomb_game_mode (Utilities|Casting|CastToBP_BombGameMode (Game|GetGameMode)))
    (Variables|/Game/GameModes/BP_BombGameMode.BP_BombGameMode_C|SetBombDiffused _asbp_bomb_game_mode true)))

(fn Lose
  (bind _asbp_bomb_game_mode (Utilities|Casting|CastToBP_BombGameMode (Game|GetGameMode)))
  (Variables|/Game/GameModes/BP_BombGameMode.BP_BombGameMode_C|SetBombExploded _asbp_bomb_game_mode true))

(fn Check
  (return true))

(fn GetHint
  (return true "Бомба" "В миссиях с условием на обезвреживание бомбы, является ключевым предметом. Для победы необходимо бомбу обязательно обезвредить. " "Нажмите Q, чтобы начать обезвреживать бомбу."))

(fn Interact
  (params (User :type BP%20Base%20Character%20Object%20Reference))
  (return true))

(fn OnBeginFocus
  (Rendering|SetVisibility (Variables|Default|GetPointLight) true false)
  (bind _asbp_base_game_mode (Utilities|Casting|CastToBP_BaseGameMode (Game|GetGameMode)))
  (Default|DisplayHint (Variables|/Game/GameModes/BP_BaseGameMode.BP_BaseGameMode_C|GetGameHUDReference _asbp_base_game_mode) self)
  (return true))

(fn OnEndFocus
  (Rendering|SetVisibility (Variables|Default|GetPointLight) false false)
  (bind _asbp_base_game_mode (Utilities|Casting|CastToBP_BaseGameMode (Game|GetGameMode)))
  (Default|HideHint (Variables|/Game/GameModes/BP_BaseGameMode.BP_BaseGameMode_C|GetGameHUDReference _asbp_base_game_mode))
  (return true))

(fn Thrust
  (params (Direction :type Vector :default "0, 0, 0") (Power :type Float%20%28single-precision%29) (Damage :type Float%20%28single-precision%29) (User :type BP%20Base%20Character%20Object%20Reference))
  (CallFunction|Explode)
  (return true))