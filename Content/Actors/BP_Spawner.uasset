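; BP_Spawner is a pad that spawns a random collectable above itself and replaces it after a delay once it is gone.
; Tick watches the current collectable; when it becomes invalid, a timer calls SpawnColletable, which picks a random class from SpawningCollectables.
; Meanwhile, a dynamic material's Alpha parameter resets to zero and interpolates at constant speed to one over the spawn time, visually showing respawn progress.
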(event EventBeginPlay
  (Variables|Default|SetAlpha 1.0)
  (Variables|Default|SetSpawnTime 5.0)
  (CallFunction|SpawnColletable))

(event EventTick
  (params (DeltaSeconds :type Float%20%28single-precision%29))
  (CallFunction|ChangeColor)
  (Utilities|IsValid (Variables|Default|GetCurrentCollectable)
    (:Is%20Not%20Valid
      (if (not (Variables|Default|GetSpawning))
        (Variables|Default|SetSpawning true)
        (Variables|Default|SetAlpha 0.0)
        (Utilities|Time|SetTimerbyFunctionName 0 "SpawnColletable" (Variables|Default|GetSpawnTime))))))

(fn ConstructionScript
  (bind _returnvalue (Rendering|Material|CreateDynamicMaterialInstance (Variables|Default|GetStaticMesh) 0 0 "None" :!class /Script/Engine.PrimitiveComponent))
  (Variables|Default|SetDynamicMaterial _returnvalue))

(fn SpawnColletable
  (bind _returnvalue (Transformation|GetActorLocation))
  (bind _spawningcollectables (Variables|Default|GetSpawningCollectables))
  (bind (_x _y _z) (Math|Vector|BreakVector _returnvalue))
  (bind _returnvalue_2 (Game|SpawnActorfromClass (Utilities|Array|Get(acopy) _spawningcollectables (Math|Random|RandomIntegerinRange 0 (- (Utilities|Array|Length _spawningcollectables) 1))) (Math|Transform|MakeTransform (Math|Vector|MakeVector _x _y (+ _z 65.0)) (Transformation|GetActorRotation)) "AdjustIfPossibleButAlwaysSpawn" self 0))
  (bind _asbp_base_collectable (Utilities|Casting|CastToBP_BaseCollectable _returnvalue_2))
  (Variables|Default|SetCurrentCollectable _asbp_base_collectable)
  (Variables|Default|SetSpawning false))

(fn ChangeColor
  (Rendering|Material|SetScalarParameterValue (Variables|Default|GetDynamicMaterial) "Alpha" (Math|Interpolation|FInterptoConstant (Variables|Default|GetAlpha) 1.0 (Utilities|Time|GetWorldDeltaSeconds) (/ 1.0 (Variables|Default|GetSpawnTime))) :!class /Script/Engine.MaterialInstanceDynamic)
  (Variables|Default|SetAlpha (Math|Interpolation|FInterptoConstant (Variables|Default|GetAlpha) 1.0 (Utilities|Time|GetWorldDeltaSeconds) (/ 1.0 (Variables|Default|GetSpawnTime)))))