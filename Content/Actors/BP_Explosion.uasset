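; BP_Explosion is a one-shot explosion actor that applies physics force, sound, AI stimuli and damage when it spawns.
; BeginPlay fires the RadialForce impulse, plays a grenade sound scaled by the game instance's volume setting, and reports a noise event.
; Characters overlapping its Sphere take fixed damage and get a damage event, with player 0 always credited as instigator.
; The actor expires after a short lifespan.
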(event EventBeginPlay
  (bind _returnvalue (Transformation|GetActorLocation))
  (Class|RadialForceComponent|FireImpulse (Variables|Default|GetRadialForce))
  (Audio|PlaySoundatLocation "/Game/Sounds/Weapons/Grenade/hegrenade-1_Cue.hegrenade-1_Cue" _returnvalue "0, 0, 0" (Variables|/Game/BP_GameInstance.BP_GameInstance_C|GetSounds (.AsBP%20Game%20Instance (Utilities|Casting|CastToBP_GameInstance (Game|GetGameInstance)))) 1.0 0.0 0 0 0)
  (Class|AISenseHearing|ReportNoiseEvent _returnvalue 2e+01 (Game|GetPlayerCharacter 0) 5e+02 "Noise")
  (bind _outactors (Collision|ComponentOverlapActors (Variables|Default|GetSphere) (Math|Transform|MakeTransform _returnvalue "0, 0, 0" "1,1,1") (Utilities|Array|MakeArray "ObjectTypeQuery1" "ObjectTypeQuery2" "ObjectTypeQuery4" "ObjectTypeQuery3") "/Game/Characters/Assets/BP_BaseCharacter.BP_BaseCharacter_C"))
  (for _array_element _outactors
    (bind _asbp_base_character (Utilities|Casting|CastToBP_BaseCharacter _array_element))
    (Default|TakeDamage _asbp_base_character 8e+01)
    (Class|AISenseDamage|ReportDamageEvent _asbp_base_character (Game|GetPlayerCharacter 0) 8e+01 (Transformation|GetActorLocation)))
  (Actor|SetLifeSpan 3.0))

(fn ConstructionScript)