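; BP_BTR is an armored personnel carrier (БТР) that serves as the drop-off point in hostage rescue missions.
; Any BP_Hostage that begins overlapping its Box is rescued.
; Focus shows a point light and a Russian HUD hint via BP_BaseGameMode, with a short retriggerable delay clearing both once focus events stop.
; Check, Interact and Thrust all return false, so it is not interactable.
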(event OnComponentBeginOverlap(Box)
  (params (OverlappedComponent :type Primitive%20Component%20Object%20Reference) (OtherActor :type Actor%20Object%20Reference) (OtherComp :type Primitive%20Component%20Object%20Reference) (OtherBodyIndex :type Integer) (bFromSweep :type Boolean) (SweepResult :type Hit%20Result%20Structure%20%28by%20ref%29))
  (bind _asbp_hostage (Utilities|Casting|CastToBP_Hostage OtherActor))
  (Default|Resque _asbp_hostage))

(event EventBeginPlay)

(event Collision|EventActorBeginOverlap
  (params (OtherActor :type Actor%20Object%20Reference)))

(event EventTick
  (params (DeltaSeconds :type Float%20%28single-precision%29)))

(event EventOnFocus
  (CallFunction|OnBeginFocus)
  (Utilities|FlowControl|RetriggerableDelay 0.1)
  (CallFunction|OnEndFocus))

(fn ConstructionScript)

(fn Check
  (return false))

(fn GetHint
  (return true "БТР" "В миссиях по освобождению заложников, чтобы спасти заложника, надо его привести к БТРу." "Нельзя взаимодействовать."))

(fn Interact
  (params (User :type BP%20Base%20Character%20Object%20Reference))
  (return false))

(fn OnBeginFocus
  (Rendering|SetVisibility (Variables|Default|GetPointLight) true false)
  (bind _asbp_base_game_mode (Utilities|Casting|CastToBP_BaseGameMode (Game|GetGameMode)))
  (Default|DisplayHint (Variables|/Game/GameModes/BP_BaseGameMode.BP_BaseGameMode_C|GetGameHUDReference _asbp_base_game_mode) self)
  (return true))

(fn OnEndFocus
  (Rendering|SetVisibility (Variables|Default|GetPointLight) false false)
  (bind _asbp_base_game_mode (Utilities|Casting|CastToBP_BaseGameMode (Game|GetGameMode)))
  (Default|HideHint (Variables|/Game/GameModes/BP_BaseGameMode.BP_BaseGameMode_C|GetGameHUDReference _asbp_base_game_mode))
  (return true))

(fn Thrust
  (params (Direction :type Vector :default "0, 0, 0") (Power :type Float%20%28single-precision%29) (Damage :type Float%20%28single-precision%29) (User :type BP%20Base%20Character%20Object%20Reference))
  (return false))